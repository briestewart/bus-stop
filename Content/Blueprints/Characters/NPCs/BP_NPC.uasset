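; Interactable NPC that runs batched dialogue from a data table and registers itself with the game instance.
; Focus toggles the player's interaction prompt; interacting locks move and look input, forces the camera onto the NPC and flags talking.
; AdvanceDialogue shows rows in a text widget, following NextDialogueID until "None"; the next call restores control.
; Later interactions resume at the table row after the last finished batch, if one exists.
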(event Custom|Event%20AdvanceDialogue
  (bind _returnvalue (Game|GetPlayerController 0))
  ;[0.15 0.15 0.15 0.5 24] Advance Dialogue
  (if (== (Variables|Default|GetCurrentDialogueID) "")
    ;;[0.15 0.15 0.15 0.5] means finished a batch of dialogue (get rid of UI, set talking to false, re-enable mouse and keyboard movement)
    (Widget|RemovefromParent (Variables|Default|GetDialogueUI))
    (Variables|Default|SetDialogueUI 0) ; SET UI to invalid
    (bind _asbp_game_instance (Utilities|Casting|CastToBP_GameInstance (Game|GetGameInstance)))
    (Variables|/Game/Blueprints/Core/BP_GameInstance.BP_GameInstance_C|SetbIsTalking _asbp_game_instance false)
    (Input|SetIgnoreLookInput _returnvalue false)
    (Input|SetIgnoreMoveInput _returnvalue false)
    (bind _asbp_player (Utilities|Casting|CastToBP_Player (Game|Player|GetPlayerPawn 0)))
    (Components|Timeline|ReversefromEnd (Variables|/Game/Blueprints/Characters/Player/BP_Player.BP_Player_C|GetForce%20Zoom%20Timeline _asbp_player))
    (Default|EventTogglenteractionUI _asbp_player false)
    (else
      ;;[0.15 0.15 0.15 0.5] else, retrieve next data row
      (bind _returnvalue_2 (Utilities|GetDataTableRow (Variables|Default|GetDialogueTable) (Variables|Default|GetCurrentDialogueID))
        (:then
          (Variables|Default|GetDialogueUI
            (:then
              _)
            (:else
              (bind _returnvalue_3 (UserInterface|CreateWidget "/Game/Blueprints/UI/WBP_DialogueText.WBP_DialogueText_C" (Game|GetPlayerController 0)))
              (bind _output_get (Variables|Default|SetDialogueUI _returnvalue_3))
              (UserInterface|Viewport|AddtoViewport _output_get 0)))
          (Rendering|Components|TextRender|SetText (Variables|/Game/Blueprints/UI/WBP_DialogueText.WBP_DialogueText_C|GetText_Dialogue (Variables|Default|GetDialogueUI)) (Utilities|Text|ToText(String) (Utilities|String|Append (.SpeakerName (Utilities|Struct|BreakS_DialogueData _returnvalue_2)) ": " (.DialogueText (Utilities|Struct|BreakS_DialogueData _returnvalue_2)))))
          (if (== (.NextDialogueID (Utilities|Struct|BreakS_DialogueData _returnvalue_2)) "")
            ;;[0.15 0.15 0.15 0.5] hit end of batch
            (Utilities|Casting|CastToBP_GameInstance (Game|GetGameInstance))
            (Variables|Default|SetLastDialogueBatchRowID (Variables|Default|GetCurrentDialogueID))
            (Variables|Default|SetCurrentDialogueID (.NextDialogueID (Utilities|Struct|BreakS_DialogueData _returnvalue_2)))
            (else
              ;;[0.15 0.15 0.15 0.5] keep going
              (Variables|Default|SetCurrentDialogueID (.NextDialogueID (Utilities|Struct|BreakS_DialogueData _returnvalue_2))))))))))

(event EventBeginPlay
  ;[0.15 0.15 0.15 0.5 24] Begin Play
  (bind _asbp_game_instance (Utilities|Casting|CastToBP_GameInstance (Game|GetGameInstance)))
  (Variables|/Game/Blueprints/Core/BP_GameInstance.BP_GameInstance_C|SetNPCRef _asbp_game_instance self))

(event Collision|EventActorBeginOverlap
  (params (OtherActor :type Actor%20Object%20Reference)))

(event EventTick
  (params (DeltaSeconds :type Float%20%28single-precision%29)))

(event EventInteract
  (bind _returnvalue (Game|GetPlayerController 0))
  (bind _returnvalue_2 (Game|GetPlayerController 0))
  (bind _lastdialoguebatchrowid (Variables|Default|GetLastDialogueBatchRowID))
  ;[0.15 0.15 0.15 0.5 24] Interact (initiate dialogue batch)
  ;;[0.15 0.15 0.15 0.5] ensures first line of dialogue is spoken before incrementing
  (if (== _lastdialoguebatchrowid "")
    (Variables|Default|SetCurrentDialogueID "Greeting")
    (bind _asbp_game_instance (Utilities|Casting|CastToBP_GameInstance (Game|GetGameInstance)))
    (Variables|/Game/Blueprints/Core/BP_GameInstance.BP_GameInstance_C|SetbIsTalking _asbp_game_instance true)
    (Input|SetIgnoreLookInput _returnvalue_2 true)
    (Input|SetIgnoreMoveInput _returnvalue_2 true)
    ;;[0.15 0.15 0.15 0.5] force look at NPC
    (bind _asbp_player (Utilities|Casting|CastToBP_Player (Game|Player|GetPlayerPawn 0)))
    (Default|EventForceLookatNPC _asbp_player)
    (Default|EventTogglenteractionUI _asbp_player true)
    (CallFunction|EventAdvanceDialogue)
    (else
      ;;[0.15 0.15 0.15 0.5] advance to new dialogue batch if next dialogue index is valid
      (bind _outrownames (DataTable|GetDataTableRowNames (Variables|Default|GetDialogueTable)))
      (if (Utilities|Array|IsValidIndex _outrownames (+ (Utilities|Array|FindItem _outrownames _lastdialoguebatchrowid) 1))
        (Variables|Default|SetCurrentDialogueID (Utilities|Array|Get(acopy) _outrownames (+ (Utilities|Array|FindItem _outrownames _lastdialoguebatchrowid) 1)))
        (bind _asbp_game_instance_2 (Utilities|Casting|CastToBP_GameInstance (Game|GetGameInstance)))
        (Variables|/Game/Blueprints/Core/BP_GameInstance.BP_GameInstance_C|SetbIsTalking _asbp_game_instance_2 true)
        (Input|SetIgnoreLookInput _returnvalue true)
        (Input|SetIgnoreMoveInput _returnvalue true)
        ;;[0.15 0.15 0.15 0.5] force look at NPC
        (bind _asbp_player_2 (Utilities|Casting|CastToBP_Player (Game|Player|GetPlayerPawn 0)))
        (Default|EventForceLookatNPC _asbp_player_2)
        (Default|EventTogglenteractionUI _asbp_player_2 true)
        (CallFunction|EventAdvanceDialogue)))))

(event EventSetFocused
  (params (bNewFocus :type Boolean))
  ;[0.15 0.15 0.15 0.5 24] NPC Focus
  (if bNewFocus
    (Development|PrintString "True" true true "(R=0.000000,G=1.000000,B=0.390245,A=1.000000)")
    (bind _asbp_player (Utilities|Casting|CastToBP_Player (Game|Player|GetPlayerPawn 0)))
    (Rendering|Components|TextRender|SetText (Variables|/Game/Blueprints/UI/WBP_InteractionPrompt.WBP_InteractionPrompt_C|GetInteractionText (Variables|/Game/Blueprints/Characters/Player/BP_Player.BP_Player_C|GetInteractionWidget _asbp_player)) (Variables|Default|GetInteractionPrompt))
    (Widget|SetVisibility (Variables|/Game/Blueprints/Characters/Player/BP_Player.BP_Player_C|GetInteractionWidget _asbp_player) "Visible")
    (Widget|SetIsEnabled (Variables|/Game/Blueprints/Characters/Player/BP_Player.BP_Player_C|GetInteractionWidget _asbp_player) true)
    (else
      (Development|PrintString "False" true true "(R=1.000000,G=0.033298,B=0.000000,A=1.000000)")
      (bind _asbp_player_2 (Utilities|Casting|CastToBP_Player (Game|Player|GetPlayerPawn 0)))
      (Widget|SetVisibility (Variables|/Game/Blueprints/Characters/Player/BP_Player.BP_Player_C|GetInteractionWidget _asbp_player_2) "Hidden")
      (Widget|SetIsEnabled (Variables|/Game/Blueprints/Characters/Player/BP_Player.BP_Player_C|GetInteractionWidget _asbp_player_2) false))))

(fn ConstructionScript)