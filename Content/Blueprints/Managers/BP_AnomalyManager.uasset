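; BP_AnomalyManager randomly decides whether an anomaly occurs in a given phase and picks which one.
; SelectAnomalyForPhase rolls against AnomalyChance, then gathers DtAnomalies data table rows whose PhaseWeight map contains that phase.
; It uses cumulative weighted random selection on those phase weights to set and return ActiveAnomaly, printing debug strings along the way.
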(fn SelectAnomalyforPhase
  (params (CurrentPhase :type Integer))
  (bind _dtanomalies (Variables|Default|GetdtAnomalies))
  (LocalVariables|SetPhase CurrentPhase)
  ;[0.15 0.15 0.15 0.5] if an anomaly will happen or not
  (if (<= (Math|Random|RandomIntegerinRange 0 100) (Variables|Default|GetAnomalyChance))
    (Development|PrintString "ANOMALY" true true "(R=0.036265,G=1.000000,B=0.000000,A=1.000000)" 5.0)
    (Utilities|FlowControl|Sequence
      (:then_0
        ;[0.15 0.15 0.15 0.5] read anomaly table and get valid anomalies for given phase
        (bind _outrownames (DataTable|GetDataTableRowNames _dtanomalies))
        (for _array_element _outrownames
          (bind _returnvalue (Utilities|GetDataTableRow _dtanomalies _array_element)
            (:then
              (if (Utilities|Map|Contains (.PhaseWeight (Utilities|Struct|BreakS_Anomaly _returnvalue)) (LocalVariables|GetPhase))
                (Utilities|Array|Add (LocalVariables|GetValidAnomalies) _returnvalue))))))
      (:then_1
        ;[0.15 0.15 0.15 0.5] loop through valid anomalies and add their weights (chances) to  'TotalWeight' accumulatively and to 'CumulativeWeight' individually
        (for _array_element_2 (LocalVariables|GetValidAnomalies)
          (Development|PrintString (.Name (Utilities|Struct|BreakS_Anomaly _array_element_2)) true true "(R=0.000000,G=0.660000,B=1.000000,A=1.000000)" 5.0)
          (bind _output_get (LocalVariables|SetTotalWeight (+ (.Value (Utilities|Map|Find (.PhaseWeight (Utilities|Struct|BreakS_Anomaly _array_element_2)) (LocalVariables|GetPhase))) (LocalVariables|GetTotalWeight))))
          (Utilities|Array|Add (LocalVariables|GetCumulativeWeight) _output_get)))
      (:then_2
        ;[0.15 0.15 0.15 0.5] loop through cumulative weights and compare random integer (0 to 'TotalWeight') to each weight to choose an anomaly
        (LocalVariables|SetRandomInt (Math|Random|RandomIntegerinRange 1 (LocalVariables|GetTotalWeight)))
        (bind (_array_element_3 _array_index) (Utilities|Array|ForEachLoopwithBreak (LocalVariables|GetCumulativeWeight) :!label _label)
          (:LoopBody
            (if (<= (LocalVariables|GetRandomInt) _array_element_3)
              (bind _output_get_2 (Variables|Default|SetActiveAnomaly (Utilities|Array|Get(acopy) (LocalVariables|GetValidAnomalies) _array_index)))
              (goto _label Break)))
          (:Completed
            (Development|PrintString (.Name (Utilities|Struct|BreakS_Anomaly _output_get_2)) true true "(R=0.385806,G=0.215770,B=1.000000,A=1.000000)" 5.0)
            (return _output_get_2)))))
    (else
      (Development|PrintString "NO ANOMALY" true true "(R=1.000000,G=0.066736,B=0.000000,A=1.000000)" 5.0)
      (return ""))))