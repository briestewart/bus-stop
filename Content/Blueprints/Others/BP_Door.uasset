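; Door actor that opens when a Player-tagged actor enters its sphere and closes after they leave.
; Sphere overlaps create and play the LS_DoorsOpen or LS_DoorsClose level sequence, with a short delay before closing.
; Four boolean state flags gate each transition, and each sequence's OnFinished callback sets the final open or closed state.
; Overlaps during a transition do not reverse it; the begin-overlap interception branch only prints debug strings.
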(event OnComponentBeginOverlap(Sphere)
  (params (OverlappedComponent :type Primitive%20Component%20Object%20Reference) (OtherActor :type Actor%20Object%20Reference) (OtherComp :type Primitive%20Component%20Object%20Reference) (OtherBodyIndex :type Integer) (bFromSweep :type Boolean) (SweepResult :type Hit%20Result%20Structure%20%28by%20ref%29))
  ;[0.15 0.15 0.15 0.5] Begin Overlap (sphere)
  (if (Actor|ActorHasTag OtherActor "Player")
    (if (Math|Boolean|ANDBoolean (not (Variables|Default|GetDoorsAreClosing)) (not (Variables|Default|GetDoorsAreOpening)) (not (Variables|Default|GetDoorsAreOpen)) (Variables|Default|GetDoorsAreClosed))
      (bind _returnvalue (Sequencer|Player|CreateLevelSequencePlayer "/Game/LevelSequences/LS_DoorsOpen.LS_DoorsOpen"))
      (bind _output_get (Variables|Default|SetCurrentLevelSequence _returnvalue))
      (Sequencer|Player|Play _output_get :!class /Script/MovieScene.MovieSceneSequencePlayer)
      (Variables|Default|SetDoorsAreOpening true)
      (Variables|Default|SetDoorsAreClosing false)
      (Variables|Default|SetDoorsAreClosed false)
      (EventDispatchers|AssignOnFinished _output_get (delegate Custom|OnFinished_Event))
      (else
        (Development|PrintString "INTERCEPT")
        (if (and (Variables|Default|GetDoorsAreClosing) (== (Variables|Default|GetCurrentLevelSequence) "/Game/LevelSequences/LS_DoorsClose.LS_DoorsClose"))
          (Development|PrintString "TRUE"))))))

(event OnComponentEndOverlap(Sphere)
  (params (OverlappedComponent :type Primitive%20Component%20Object%20Reference) (OtherActor :type Actor%20Object%20Reference) (OtherComp :type Primitive%20Component%20Object%20Reference) (OtherBodyIndex :type Integer))
  ;[0.15 0.15 0.15 0.5] End Overlap (sphere)
  (if (Actor|ActorHasTag OtherActor "Player")
    (if (Math|Boolean|ANDBoolean (not (Variables|Default|GetDoorsAreOpening)) (not (Variables|Default|GetDoorsAreClosing)) (not (Variables|Default|GetDoorsAreClosed)) (Variables|Default|GetDoorsAreOpen))
      (Utilities|FlowControl|Delay 2.0)
      (bind _returnvalue (Sequencer|Player|CreateLevelSequencePlayer "/Game/LevelSequences/LS_DoorsClose.LS_DoorsClose"))
      (bind _output_get (Variables|Default|SetCurrentLevelSequence _returnvalue))
      (Sequencer|Player|Play _output_get :!class /Script/MovieScene.MovieSceneSequencePlayer)
      (Variables|Default|SetDoorsAreClosing true)
      (Variables|Default|SetDoorsAreOpening false)
      (Variables|Default|SetDoorsAreOpen false)
      (EventDispatchers|AssignOnFinished _output_get (delegate Custom|OnFinished_Event_0)))))

(event Custom|OnFinished_Event
  ;[0.15 0.15 0.15 0.5] On Door Open Finish
  (Variables|Default|SetDoorsAreOpening false)
  (Variables|Default|SetDoorsAreOpen true))

(event Custom|OnFinished_Event_0
  ;[0.15 0.15 0.15 0.5] On Door Close Finish
  (Variables|Default|SetDoorsAreClosing false)
  (Variables|Default|SetDoorsAreClosed true))

(event EventBeginPlay)

(event Collision|EventActorBeginOverlap
  (params (OtherActor :type Actor%20Object%20Reference)))

(event EventTick
  (params (DeltaSeconds :type Float%20%28single-precision%29)))

(fn ConstructionScript)