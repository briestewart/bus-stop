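; Automatic double door that opens when a Player-tagged actor enters its sphere and closes on a timer after the player leaves.
; A DoorState enum gates the overlap logic, with level sequences playing the normal open and close motions.
; Re-entry clears the close timer; if already closing, it stops the sequence and a timeline lerps both doors from their current positions to the open offsets.
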(event OnComponentBeginOverlap(Sphere)
  (params (OverlappedComponent :type Primitive%20Component%20Object%20Reference) (OtherActor :type Actor%20Object%20Reference) (OtherComp :type Primitive%20Component%20Object%20Reference) (OtherBodyIndex :type Integer) (bFromSweep :type Boolean) (SweepResult :type Hit%20Result%20Structure%20%28by%20ref%29))
  ;[0.15 0.15 0.15 0.5] Begin Overlap (sphere)
  (if (Actor|ActorHasTag OtherActor "Player")
    (Variables|Default|SetPlayerInOverlap true)
    (Utilities|Time|ClearandInvalidateTimerbyHandle (Variables|Default|GetCloseDoorHandle))
    (Utilities|FlowControl|Sequence
      (:then_0
        (if (Utilities|Enum|Equal(Enum) (Utilities|String|EnumtoString (Variables|Default|GetDoorState)) "Closed")
          (Variables|Default|SetDoorState "NewEnumerator3")
          (bind _returnvalue (Sequencer|Player|CreateLevelSequencePlayer "/Game/LevelSequences/LS_DoorsOpen.LS_DoorsOpen"))
          (bind _output_get (Variables|Default|SetCurrentLevelSequence _returnvalue))
          (Sequencer|Player|Play _output_get :!class /Script/MovieScene.MovieSceneSequencePlayer)
          (EventDispatchers|AssignOnFinished _returnvalue (delegate Custom|OnFinishedOpening))))
      (:then_1
        (if (Utilities|Enum|Equal(Enum) (Utilities|String|EnumtoString (Variables|Default|GetDoorState)) "Closing")
          (Variables|Default|SetDoorState "NewEnumerator3")
          (Sequencer|Player|Stop (Variables|Default|GetCurrentLevelSequence) :!class /Script/MovieScene.MovieSceneSequencePlayer)
          (Audio|Components|Audio|Play (Variables|Default|GetClosingToOpening) 1.0)
          (Variables|Default|SetLeftDoorRelativeLocation (.location (Transformation|GetRelativeTransform (Variables|Default|GetLeftDoor))))
          (Variables|Default|SetRightDoorRelativeLocation (.location (Transformation|GetRelativeTransform (Variables|Default|GetRightDoor))))
          (bind _newtrack_0 (Timeline|ReverseDoors PlayFromStart)
            (:Update
              (Transformation|SetRelativeLocation (Variables|Default|GetLeftDoor) (Math|Vector|Lerp(Vector) (Variables|Default|GetLeftDoorRelativeLocation) (Variables|Default|GetLeftDoorOpenLocation) _newtrack_0) false false)
              (Transformation|SetRelativeLocation (Variables|Default|GetRightDoor) (Math|Vector|Lerp(Vector) (Variables|Default|GetRightDoorRelativeLocation) (Variables|Default|GetRightDoorOpenLocation) _newtrack_0) false false))
            (:Finished
              (Audio|Components|Audio|Stop (Variables|Default|GetClosingToOpening))
              (Variables|Default|SetDoorState "NewEnumerator2"))))))))

(event OnComponentEndOverlap(Sphere)
  (params (OverlappedComponent :type Primitive%20Component%20Object%20Reference) (OtherActor :type Actor%20Object%20Reference) (OtherComp :type Primitive%20Component%20Object%20Reference) (OtherBodyIndex :type Integer))
  ;[0.15 0.15 0.15 0.5] End Overlap (sphere)
  (if (Actor|ActorHasTag OtherActor "Player")
    (Variables|Default|SetPlayerInOverlap false)
    (Utilities|FlowControl|Sequence
      (:then_0
        (if (Utilities|Enum|Equal(Enum) (Utilities|String|EnumtoString (Variables|Default|GetDoorState)) "Opened")
          (bind _returnvalue (Utilities|Time|SetTimerbyFunctionName 0 "CloseDoor" 2.0))
          (Variables|Default|SetCloseDoorHandle _returnvalue)))
      (:then_1
        (if (Utilities|Enum|Equal(Enum) (Utilities|String|EnumtoString (Variables|Default|GetDoorState)) "Opening")
          (bind _returnvalue_2 (Utilities|Time|SetTimerbyFunctionName 0 "CloseDoor" 3.5))
          (Variables|Default|SetCloseDoorHandle _returnvalue_2))))))

(event Custom|OnFinishedOpening
  ;[0.15 0.15 0.15 0.5] Begin Overlap (sphere)
  ;;[0.15 0.15 0.15 0.5] On Door Open Finish
  (Variables|Default|SetDoorState "NewEnumerator2"))

(event Custom|OnFinishedClosing
  ;[0.15 0.15 0.15 0.5] End Overlap (sphere)
  ;;[0.15 0.15 0.15 0.5] On Door Close Finish
  (Variables|Default|SetDoorState "NewEnumerator0"))

(event EventBeginPlay)

(event Collision|EventActorBeginOverlap
  (params (OtherActor :type Actor%20Object%20Reference)))

(event EventTick
  (params (DeltaSeconds :type Float%20%28single-precision%29)))

(fn ConstructionScript)

(fn CloseDoor
  (if (not (Variables|Default|GetPlayerInOverlap))
    (Variables|Default|SetDoorState "NewEnumerator1")
    (bind _returnvalue (Sequencer|Player|CreateLevelSequencePlayer "/Game/LevelSequences/LS_DoorsClose.LS_DoorsClose"))
    (bind _output_get (Variables|Default|SetCurrentLevelSequence _returnvalue))
    (Sequencer|Player|Play _output_get :!class /Script/MovieScene.MovieSceneSequencePlayer)
    (EventDispatchers|BindEventtoOnFinished _output_get (EventDispatchers|CreateEvent :!event Custom|OnFinishedClosing))))