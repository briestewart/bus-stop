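; BP_Bus is an interactable bus that drives to and from a stop as part of game progression.
; It binds arrival and departure to BP_GameInstance events, using timelines to lerp between start, stop and end locations.
; Interacting marks the player aboard and reports EnterBus; an arrival with the player aboard reports ExitBus after a delay.
; Departure starts after a delay and, once finished, sets BusArrival and triggers the game instance's event check.
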(event Custom|Event%20BusArrival
  ;[0.15 0.15 0.15 0.5 24] Bus Arrival
  (bind _cometrack (Timeline|Bus%20Coming%20Timeline PlayFromStart)
    (:Update
      (Transformation|SetActorLocation (Math|Vector|Lerp(Vector) (Variables|Default|GetStartLocation) (Variables|Default|GetBusStopLocation) _cometrack) false false))
    (:Finished
      (if (Variables|Default|GetbPlayerIsOnBus)
        (Utilities|FlowControl|Delay 5.0)
        (Variables|Default|SetbPlayerIsOnBus false)
        (bind _asbp_game_instance (Utilities|Casting|CastToBP_GameInstance (Game|GetGameInstance)))
        (Default|UpdateGameProgressState _asbp_game_instance "ExitBus")
        (Default|CheckandTriggerEvent _asbp_game_instance)))))

(event Custom|Event%20BusDeparture
  ;[0.15 0.15 0.15 0.5 24] Bus Departure
  (Utilities|FlowControl|Delay 5.0)
  (bind _leavetrack (Timeline|Bus%20Leaving%20Timeline PlayFromStart)
    (:Update
      (Transformation|SetActorLocation (Math|Vector|Lerp(Vector) (Variables|Default|GetBusStopLocation) (Variables|Default|GetEndLocation) _leavetrack) false false))
    (:Finished
      (bind _asbp_game_instance (Utilities|Casting|CastToBP_GameInstance (Game|GetGameInstance)))
      (Default|UpdateGameProgressState _asbp_game_instance "BusArrival")
      (Default|CheckandTriggerEvent _asbp_game_instance))))

(event EventBeginPlay
  ;[0.15 0.15 0.15 0.5 24] Begin Play
  (bind _asbp_game_instance (Utilities|Casting|CastToBP_GameInstance (Game|GetGameInstance)))
  (EventDispatchers|BindEventtoMakeBusArrive _asbp_game_instance (delegate Custom|Event%20BusArrival))
  (EventDispatchers|BindEventtoMakeBusDepart _asbp_game_instance (delegate Custom|Event%20BusDeparture)))

(event Collision|EventActorBeginOverlap
  (params (OtherActor :type Actor%20Object%20Reference)))

(event EventTick
  (params (DeltaSeconds :type Float%20%28single-precision%29)))

(event EventInteract
  ;[0.15 0.15 0.15 0.5 24] Interact
  (bind _asbp_game_instance (Utilities|Casting|CastToBP_GameInstance (Game|GetGameInstance)))
  (Default|UpdateGameProgressState _asbp_game_instance "EnterBus")
  (Variables|Default|SetbPlayerIsOnBus true)
  (Default|CheckandTriggerEvent _asbp_game_instance))

(fn ConstructionScript)