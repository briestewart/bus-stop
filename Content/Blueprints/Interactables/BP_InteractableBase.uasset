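; Base interactable actor that shows a prompt on the player's interaction widget when focused and glows when interacted with.
; SetFocused casts the player pawn to BP_Player, then either fills in InteractionPrompt and shows its widget or hides and disables it.
; Interact_1 applies a new dynamic glow material to the mesh and raises GlowIntensity; its comment marks it as possibly pending deletion.
; Both events still print debug strings.
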(event Custom|Interact_1
  ;[0.15 0.15 0.15 0.5] Glow on Sight (pending delete?)
  (Development|PrintString "Interacted with object!")
  (bind _returnvalue (Rendering|Material|CreateDynamicMaterialInstance "/Game/Materials/M_InteractableGlow.M_InteractableGlow" "None" "None" :!class /Script/Engine.KismetMaterialLibrary))
  (bind _output_get (Variables|Default|SetDynamicMaterialInstance _returnvalue))
  (Rendering|Material|SetMaterial (Variables|Default|GetMesh) 0 _output_get)
  (Rendering|Material|SetScalarParameterValueonMaterials (Variables|Default|GetMesh) "GlowIntensity" 1.0))

(event EventBeginPlay)

(event Collision|EventActorBeginOverlap
  (params (OtherActor :type Actor%20Object%20Reference)))

(event EventTick
  (params (DeltaSeconds :type Float%20%28single-precision%29)))

(event EventSetFocused
  (params (bNewFocus :type Boolean))
  ;[0.15 0.15 0.15 0.5 24] Item Focus
  (if bNewFocus
    (Development|PrintString "True" true true "(R=0.000000,G=1.000000,B=0.390245,A=1.000000)")
    (bind _asbp_player (Utilities|Casting|CastToBP_Player (Game|Player|GetPlayerPawn 0)))
    (Rendering|Components|TextRender|SetText (Variables|/Game/Blueprints/UI/WBP_InteractionPrompt.WBP_InteractionPrompt_C|GetInteractionText (Variables|/Game/Blueprints/Characters/Player/BP_Player.BP_Player_C|GetInteractionWidget _asbp_player)) (Variables|Default|GetInteractionPrompt))
    (Widget|SetVisibility (Variables|/Game/Blueprints/Characters/Player/BP_Player.BP_Player_C|GetInteractionWidget _asbp_player) "Visible")
    (Widget|SetIsEnabled (Variables|/Game/Blueprints/Characters/Player/BP_Player.BP_Player_C|GetInteractionWidget _asbp_player) true)
    (else
      (Development|PrintString "False" true true "(R=1.000000,G=0.033298,B=0.000000,A=1.000000)")
      (bind _asbp_player_2 (Utilities|Casting|CastToBP_Player (Game|Player|GetPlayerPawn 0)))
      (Widget|SetVisibility (Variables|/Game/Blueprints/Characters/Player/BP_Player.BP_Player_C|GetInteractionWidget _asbp_player_2) "Hidden")
      (Widget|SetIsEnabled (Variables|/Game/Blueprints/Characters/Player/BP_Player.BP_Player_C|GetInteractionWidget _asbp_player_2) false))))

(fn ConstructionScript)