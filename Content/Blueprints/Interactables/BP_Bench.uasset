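; BP_Bench is an interactable bench that records the player's forward (no anomaly) or backward (anomaly) choice while they are leaving the store.
; Interact reads the bench's actor tag, sets the selection and on-bench flags in BP_GameInstance, then updates game progress and triggers its event check.
; Forward benches also run DetermineBenchView, which uses a dot product against the bench's right vector to store the player's approach side.
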(event EventInteract
  ;[0.15 0.15 0.15 0.5 24] Interact
  (bind _asbp_game_instance (Utilities|Casting|CastToBP_GameInstance (Game|GetGameInstance)))
  (bind _output_get (Variables|Default|SetGameRef _asbp_game_instance))
  (if (and (Variables|/Game/Blueprints/Core/BP_GameInstance.BP_GameInstance_C|GetbIsPlayerLeavingStore _output_get) (not (Variables|/Game/Blueprints/Core/BP_GameInstance.BP_GameInstance_C|GetbIsPlayerOnBench _output_get)))
    (if (Actor|ActorHasTag "benchForward")
      (Variables|/Game/Blueprints/Core/BP_GameInstance.BP_GameInstance_C|SetbSelectedForward (Variables|Default|GetGameRef) true)
      (Variables|/Game/Blueprints/Core/BP_GameInstance.BP_GameInstance_C|SetbSelectedBackward (Variables|Default|GetGameRef) false)
      (Variables|/Game/Blueprints/Core/BP_GameInstance.BP_GameInstance_C|SetbIsPlayerOnBench (Variables|Default|GetGameRef) true)
      (Development|PrintString "Going Forward (no anomaly)" true true "(R=0.911088,G=1.000000,B=0.057292,A=1.000000)" 5.0)
      (CallFunction|DetermineBenchView)
      (Default|UpdateGameProgressState (Variables|Default|GetGameRef) "GetOnBench")
      (Default|CheckandTriggerEvent (Variables|Default|GetGameRef))
      (elif (Actor|ActorHasTag "benchBackward")
        (Variables|/Game/Blueprints/Core/BP_GameInstance.BP_GameInstance_C|SetbSelectedBackward (Variables|Default|GetGameRef) true)
        (Variables|/Game/Blueprints/Core/BP_GameInstance.BP_GameInstance_C|SetbSelectedForward (Variables|Default|GetGameRef) false)
        (Variables|/Game/Blueprints/Core/BP_GameInstance.BP_GameInstance_C|SetbIsPlayerOnBench (Variables|Default|GetGameRef) true)
        (Development|PrintString "Going Backward (anomaly)" true true "(R=0.000000,G=1.000000,B=0.557249,A=1.000000)" 5.0)
        (Default|UpdateGameProgressState (Variables|Default|GetGameRef) "GetOnBench")
        (Default|CheckandTriggerEvent (Variables|Default|GetGameRef))))))

(fn ConstructionScript)

(fn DetermineBenchView
  (bind _gameref (Variables|Default|GetGameRef))
  (if (> (Math|Vector|DotProduct (Math|Vector|Normalize (- (Transformation|GetActorLocation (Game|Player|GetPlayerPawn 0)) (Transformation|GetActorLocation))) (Transformation|GetActorRightVector)) 0.0)
    (Development|PrintString "Right side" true true "(R=0.406250,G=1.000000,B=0.482107,A=1.000000)")
    (Variables|/Game/Blueprints/Core/BP_GameInstance.BP_GameInstance_C|SetApproachBenchFromRight _gameref true)
    (Variables|/Game/Blueprints/Core/BP_GameInstance.BP_GameInstance_C|SetApproachBenchFromLeft _gameref false)
    (else
      (Development|PrintString "Left side" true true "(R=0.627147,G=0.494792,B=1.000000,A=1.000000)")
      (Variables|/Game/Blueprints/Core/BP_GameInstance.BP_GameInstance_C|SetApproachBenchFromRight _gameref false)
      (Variables|/Game/Blueprints/Core/BP_GameInstance.BP_GameInstance_C|SetApproachBenchFromLeft _gameref true))))